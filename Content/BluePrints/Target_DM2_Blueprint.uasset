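; Destructible target that replaces itself with an intact copy some time after it is broken.
; Fracturing the DestructibleComponent starts a countdown that Tick decrements once per frame, so the delay depends on frame rate.
; When it runs out, the actor spawns a new instance of its own class at its location, copies its rotation onto it, then destroys itself.
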(event `self.ReceiveTick`
  (params (DeltaSeconds :type "Float (single-precision)"))
  (if (!= (`self.respawntimer`) -1)
    (set `self.respawntimer` (- (`self.respawntimer`) 1))
    (if (<= (`self.respawntimer`) 0)
      (bind _returnvalue (`|SpawnActorFromClass` "Target_DM2_Blueprint_C" (`KismetMathLibrary.Conv_VectorToTransform` (`self.K2_GetActorLocation`)) "Undefined" "OverrideRootScale"))
      (`self.K2_SetActorRotation` _returnvalue (`self.K2_GetActorRotation`) false)
      (`self.K2_DestroyActor`))))

(event `self.DestructibleComponent.OnComponentFracture`
  (params (HitPoint :type "Vector Structure (by ref)") (HitDirection :type "Vector Structure (by ref)"))
  (set `self.respawntimer` 300))

(fn `UserConstructionScript`)